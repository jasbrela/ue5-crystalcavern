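; BP_VictoryZone is a level exit that advances the game when the player pawn overlaps it.
; It checks for remaining BP_Collectible actors, but both branches are empty, so the level completes either way.
; Completion finds the current level in the LevelNames array and opens the next one, wrapping to the first after the last.
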(event `self.ReceiveActorBeginOverlap`
  (params (OtherActor :type "Actor Object Reference"))
  (`/Game/Blueprints/Libraries/CC_MacroLibrary.Is Player Pawn` OtherActor
    (:`Is Player`
      (if (`self.Any Remaining Crystal`)
        _
        (else
          _))
      (`self.Complete Level`))))

(fn `Any Remaining Crystal`
  (returns (`Return Value` :type Boolean))
  (bind _outactors (`GameplayStatics.GetAllActorsOfClass` "/Game/Blueprints/BP_Collectible.BP_Collectible_C"))
  (return (> (`KismetArrayLibrary.Array_Length` _outactors) 0)))

(fn `Complete Level`
  (bind _return_value (`self.Is Last Level`))
  (if _return_value
    (`self.Load First Level`)
    (else
      (`self.Load Next Level`))))

(fn `Get Current Level Index`
  (returns (Index :type Integer))
  (bind _returnvalue (`GameplayStatics.GetCurrentLevelName` true))
  (return (`KismetArrayLibrary.Array_Find` (`self.LevelNames`) (`KismetStringLibrary.Conv_StringToName` _returnvalue))))

(fn `Is Last Level`
  (returns (`Return Value` :type Boolean))
  (return (== (`KismetArrayLibrary.Array_LastIndex` (`self.LevelNames`)) (`self.Get Current Level Index`))))

(fn `Load First Level`
  (`GameplayStatics.OpenLevel` (`|GetArrayItem` (`self.LevelNames`))))

(fn `Load Next Level`
  (`GameplayStatics.OpenLevel` (`|GetArrayItem` (`self.LevelNames`) (+ (`self.Get Current Level Index`) 1))))

(fn `UserConstructionScript`)