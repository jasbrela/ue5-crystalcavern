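; BP_Cannon is an automatic cannon actor that repeatedly fires projectiles with an animated barrel.
; After an initial delay on BeginPlay, it waits for the firing rate, then spawns a BP_Projectile at the Arrow component's location and rotation.
; The FiringAnimation timeline slides the barrel along its local Y axis from its starting position.
; The timeline's Cannon Fired event track re-enters the delay, closing the firing loop.
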(event `self.ReceiveBeginPlay`
  (bind _cannon_barrel (`self.Cannon Barrel`))
  (bind (_relativelocation_x _relativelocation_y) (`KismetMathLibrary.BreakVector` (`SceneComponent.RelativeLocation` (`self.Cannon Barrel`))))
  (bind (_relativelocation_x_2 _relativelocation_y_2 _relativelocation_z) (`KismetMathLibrary.BreakVector` (`SceneComponent.RelativeLocation` _cannon_barrel)))
  (set `self.StartLocalY` _relativelocation_y)
  (`KismetSystemLibrary.Delay` (`self.DelayBeforeFirstFire`))
  (`KismetSystemLibrary.Delay` (`self.Firing Rate`) :!label _label)
  (`self.SpawnProjectile`)
  (bind (_direction _firing_alpha) (`Timeline|Firing Animation` :!via `PlayFromStart`)
    (:`Update`
      (`SceneComponent.K2_SetRelativeLocation` _cannon_barrel (`KismetMathLibrary.MakeVector` _relativelocation_x_2 (`KismetMathLibrary.MapRangeUnclamped` _firing_alpha 0.0 1.0 (`self.StartLocalY`) -24.0) _relativelocation_z) false false))
    (:`Cannon Fired`
      (goto _label))))

(fn `SpawnProjectile`
  (bind _arrow (`self.Arrow`))
  (`|SpawnActorFromClass` "/Game/Blueprints/BP_Projectile.BP_Projectile_C" (`KismetMathLibrary.MakeTransform` (`SceneComponent.K2_GetComponentLocation` _arrow) (`SceneComponent.K2_GetComponentRotation` _arrow)) "Undefined" "MultiplyWithRoot" null null))

(fn `UserConstructionScript`)