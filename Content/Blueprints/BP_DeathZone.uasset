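; BP_DeathZone is a kill volume that restarts the current level when the player enters it.
; On BeginPlay it fades the camera in from black.
; When the player pawn overlaps its Trigger component, it fades the screen out, waits for the fade to finish, then reopens the current level by name.
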(event `self.ReceiveBeginPlay`
  ;[0.4567 0.4791 1] Fade-in
  (`PlayerCameraManager.StartCameraFade` :`self` (`GameplayStatics.GetPlayerCameraManager` 0) :`FromAlpha` 1.0 :`ToAlpha` 0.0 :`Duration` 0.5 :`bHoldWhenFinished` true))

(event `self.Trigger.OnComponentBeginOverlap`
  (params (OverlappedComponent :type "PrimitiveComponent Object Reference") (OtherActor :type "Actor Object Reference") (OtherComp :type "PrimitiveComponent Object Reference") (OtherBodyIndex :type Integer) (bFromSweep :type Boolean) (SweepResult :type "HitResult Structure (by ref)"))
  ;[0.2686 1 0.5645] Fade-out
  (if (== OtherActor (`GameplayStatics.GetPlayerPawn` 0))
    (`PlayerCameraManager.StartCameraFade` :`self` (`GameplayStatics.GetPlayerCameraManager` 0) :`ToAlpha` 1.0 :`Duration` 0.5 :`bHoldWhenFinished` true)
    (`KismetSystemLibrary.Delay` 0.5)
    ;[1 0.1354 0.1354] Restart Level
    (bind _returnvalue (`GameplayStatics.GetCurrentLevelName` true))
    (`GameplayStatics.OpenLevel` (`KismetStringLibrary.Conv_StringToName` _returnvalue))))

(fn `UserConstructionScript`)