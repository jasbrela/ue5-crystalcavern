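; Collectible pickup that bobs and spins, then flies into the player and is destroyed.
; IdleTimeline drives the float from the stored start position, with odd-flagged instances first offset and rotated to vary the motion.
; Player overlap, or IdleTimeline finishing, plays CollectTimeline, which lerps the actor to the player's live position while shrinking it.
; The intended light fade uses a fixed zero alpha, so intensity stays at its initial value.
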(event `self.ReceiveBeginPlay`
  (`self.IsOdd`
    (:`Odd`
      (`self.FlipAnimation`))
    (:`Even`
      _))
  (`self.StoreInitialValues`)
  (bind (_direction _floatingalpha) (`Timeline|IdleTimeline`)
    (:`Update`
      (`self.PlayFloatingAnimation` _floatingalpha (`self.LerpStartPosition`)))
    (:`Finished`
      (bind (_direction_2 _movementalpha _lightingalpha) (`Timeline|CollectTimeline` :!label _label)
        (:`Update`
          (`self.MoveToPlayer` _movementalpha)
          (`self.AdjustLightIntensity` _lightingalpha))
        (:`Finished`
          (`self.K2_DestroyActor`))))))

(event `self.Collision.OnComponentBeginOverlap`
  (params (OverlappedComponent :type "PrimitiveComponent Object Reference") (OtherActor :type "Actor Object Reference") (OtherComp :type "PrimitiveComponent Object Reference") (OtherBodyIndex :type Integer) (bFromSweep :type Boolean) (SweepResult :type "HitResult Structure (by ref)"))
  (`self.IsPlayerPawn` OtherActor
    (:`Is Player`
      (goto _label))))

(fn `AdjustLightIntensity`
  (params (InputPin :type "Float (single-precision)"))
  (`LightComponent.SetIntensity` (`self.PointLight`) (`KismetMathLibrary.Lerp` (`self.LightStartIntensity`))))

(fn `FlipAnimation`
  (`self.K2_SetActorLocation` (+ (`self.K2_GetActorLocation`) (`KismetMathLibrary.MakeVector` 0.0 0.0 (`self.ZOffset`))))
  (bind _result (`/Engine/EditorBlueprintResources/StandardMacros.NegateFloat` (`self.ZOffset`))
    (:`  `
      (set `self.ZOffset` _result)
      (`self.K2_AddActorWorldRotation` (`KismetMathLibrary.MakeRotator` 0.0 0.0 (`self.ZRotationOffset`))))))

(fn `MoveToPlayer`
  (params (`Movement Alpha` :type "Float (single-precision)"))
  (`self.K2_SetActorLocation` (`KismetMathLibrary.VLerp` (`self.LerpStartPosition`) (`self.K2_GetActorLocation` (`GameplayStatics.GetPlayerPawn` 0)) `Movement Alpha`))
  (`self.SetActorScale3D` (`KismetMathLibrary.VLerp` (1.0 1.0 1.0) (0.0 0.0 0.0) `Movement Alpha`)))

(fn `PlayFloatingAnimation`
  (params (Alpha :type "Float (single-precision)") (InputPin :type "Vector Structure"))
  (`self.K2_SetActorLocation` (`KismetMathLibrary.VLerp` InputPin (+ InputPin (`KismetMathLibrary.MakeVector` 0.0 0.0 (`self.ZOffset`))) Alpha))
  (`self.K2_AddActorLocalRotation` (`KismetMathLibrary.MakeRotator` 0.0 0.0 (`self.ZRotationOffset`))))

(fn `StoreInitialValues`
  (set `self.LerpStartPosition` (`self.K2_GetActorLocation`))
  (set `self.LightStartIntensity` (`LightComponentBase.Intensity` (`self.PointLight`))))

(fn `UserConstructionScript`)