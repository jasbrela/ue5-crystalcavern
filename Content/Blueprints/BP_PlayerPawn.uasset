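; BP_PlayerPawn is a player-controlled pawn that moves by applying physics torque to its mesh.
; On BeginPlay it adds the CristalCavern_InputMapping Enhanced Input context to its player controller's local subsystem.
; The forward and right input actions apply torque around world X and Y respectively, scaled by AccelerationMultiplier.
; The torque is applied as an acceleration change, so the mesh's mass does not affect the response.
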(event `self.ReceiveBeginPlay`
  ;[0.3068 0.2957 0.4896] Mapping Context
  (bind _asplayer_controller (cast `PlayerController` (`self.GetController`)))
  (bind _returnvalue (pcsubsystem `EnhancedInputLocalPlayerSubsystem` _asplayer_controller))
  (`/Engine/EditorBlueprintResources/StandardMacros.IsValid` _returnvalue
    (:`Is Valid`
      (`EnhancedInputSubsystemInterface.AddMappingContext` _returnvalue "/Game/Input/CristalCavern_InputMapping.CristalCavern_InputMapping" 0 (struct)))))

(event `EnhancedInput|/Game/Input/IA_MoveForward`
  (params (ActionValue :type "Float (double-precision)") (ElapsedSeconds :type "Float (double-precision)") (TriggeredSeconds :type "Float (double-precision)") (InputAction :type "InputAction Object Reference" :default "/Game/Input/IA_MoveForward.IA_MoveForward"))
  ;[0.8399 0.3906 1] Player Movement
  (:`Triggered`
    (`PrimitiveComponent.AddTorqueInRadians` (`self.Mesh`) (`KismetMathLibrary.MakeVector` (* ActionValue (`self.Acceleration Multiplier`))) "None" true)))

(event `EnhancedInput|/Game/Input/IA_MoveRight`
  (params (ActionValue :type "Float (double-precision)") (ElapsedSeconds :type "Float (double-precision)") (TriggeredSeconds :type "Float (double-precision)") (InputAction :type "InputAction Object Reference" :default "/Game/Input/IA_MoveRight.IA_MoveRight"))
  ;[0.8399 0.3906 1] Player Movement
  (:`Triggered`
    (`PrimitiveComponent.AddTorqueInRadians` (`self.Mesh`) (`KismetMathLibrary.MakeVector` 0.0 (* ActionValue (`self.Acceleration Multiplier`))) "None" true)))

(fn `UserConstructionScript`)